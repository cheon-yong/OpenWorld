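; BP_Minimap is the driver for the player minimap, creating the WBG_Minimap widget and adding it to the viewport on BeginPlay.
; Every Tick it writes the player character's location and yaw into the MP_Minimap material parameter collection.
; Location is passed as a vector parameter, while negative yaw is wrapped by 360 degrees and divided down to a 0–1 scalar.
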(event `self.ReceiveBeginPlay`
  (bind _returnvalue (`|CreateWidget` "/Game/Minimap/WBG_Minimap.WBG_Minimap_C"))
  (`UserWidget.AddToViewport` _returnvalue 0))

(event `self.ReceiveTick`
  (params (DeltaSeconds :type "Float (single-precision)"))
  (bind _returnvalue (`GameplayStatics.GetPlayerCharacter` 0))
  (bind (_returnvalue_roll _returnvalue_pitch _returnvalue_yaw) (`KismetMathLibrary.BreakRotator` (`self.K2_GetActorRotation` _returnvalue)))
  (`KismetMaterialLibrary.SetVectorParameterValue` "/Game/Minimap/MP_Minimap.MP_Minimap" "Player Location" (`KismetMathLibrary.Conv_VectorToLinearColor` (`self.K2_GetActorLocation` _returnvalue)))
  (`KismetMaterialLibrary.SetScalarParameterValue` "/Game/Minimap/MP_Minimap.MP_Minimap" "Player Yaw" (/ (`KismetMathLibrary.SelectFloat` (+ _returnvalue_yaw 360.0) _returnvalue_yaw (< _returnvalue_yaw 0.0)) 360.0)))

(fn `UserConstructionScript`)